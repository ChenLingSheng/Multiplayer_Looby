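; PC_Lobby is the lobby player controller that sets up the lobby UI and spawns the player's character.
; On BeginPlay, the local controller shows the UMG_Lobby widget and mouse cursor, then passes the player name from GI_Main to a spawn event.
; That event spawns a PCH_Game at a PlayerStart, assigns the name and a PlayerID concatenated from the current date and time, and possesses it.
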(event `self.ReceiveBeginPlay`
  (if (`self.IsLocalPlayerController`)
    (bind _returnvalue (`|CreateWidget` "/Game/MyAssets/UMG/UMG_Lobby.UMG_Lobby_C" self))
    (`UserWidget.AddToViewport` _returnvalue 0)
    (set `self.bShowMouseCursor` true)
    (bind _asgi_main (cast `/Game/MyAssets/Gamepley/GI_Main` (`GameplayStatics.GetGameInstance`)))
    (`self.EVE_Spawn_Player` (`/Game/MyAssets/Gamepley/GI_Main.PlayerName` _asgi_main))))

(event `EVE_Spawn_Player`
  (params (PlayerName :type Text))
  (bind (_returnvalue_year _returnvalue_month _returnvalue_day _returnvalue_hour _returnvalue_minute _returnvalue_second _returnvalue_millisecond) (`KismetMathLibrary.BreakDateTime` (`KismetMathLibrary.Now`)))
  (bind _returnvalue (`GameplayStatics.GetActorOfClass` "/Script/Engine.PlayerStart"))
  (bind _returnvalue_2 (`|SpawnActorFromClass` "/Game/MyAssets/Gamepley/PCH_Game.PCH_Game_C" (`self.GetTransform` _returnvalue) "Undefined" "OverrideRootScale" null PlayerName (`KismetStringLibrary.Concat_StrStr` (`KismetStringLibrary.Conv_IntToString` _returnvalue_year) (`KismetStringLibrary.Conv_IntToString` _returnvalue_month) (`KismetStringLibrary.Conv_IntToString` _returnvalue_day) (`KismetStringLibrary.Conv_IntToString` _returnvalue_hour) (`KismetStringLibrary.Conv_IntToString` _returnvalue_minute) (`KismetStringLibrary.Conv_IntToString` _returnvalue_second) (`KismetStringLibrary.Conv_IntToString` _returnvalue_millisecond)) null))
  (`self.Possess` self _returnvalue_2))

(fn `UserConstructionScript`)